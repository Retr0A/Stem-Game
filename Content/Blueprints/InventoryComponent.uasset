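; Inventory component that adds items to the player's inventory menu as slot widgets.
; AddItem creates an InvSlotItem widget from the item structure and adds it to the ItemsGrid, reached through player 0's MainController UI.
; Row and column counters track the next free cell, wrapping to a new row after eight columns.
; It keeps no item list of its own and has no removal logic.
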(event EventBeginPlay)

(event EventTick
  (params (DeltaSeconds :type Float%20%28single-precision%29)))

(fn AddItem
  (params (ItemStructure :type Item%20Structure%20Structure))
  (bind _returnvalue (UserInterface|CreateWidget "/Game/UI/Inventory/InvSlotItem.InvSlotItem_C" 0 ItemStructure))
  (Class|GridPanel|AddChildtoGrid (Variables|/Game/UI/Inventory/InventoryMenu.InventoryMenu_C|GetItemsGrid (Variables|/Game/UI/MenuUI.MenuUI_C|GetInventoryMenu (Variables|/Game/UI/DisplayUI.DisplayUI_C|GetMenuUI (Variables|/Game/Blueprints/MainController.MainController_C|GetDisplayUI (.AsMain%20Controller (Utilities|Casting|CastToMainController (Game|GetPlayerController 0))))))) _returnvalue (Variables|Default|GetCurrentFreeRowSlot) (Variables|Default|GetCurrentFreeColumnSlot))
  (if (== (Variables|Default|GetCurrentFreeColumnSlot) 7)
    (Variables|Default|SetCurrentFreeColumnSlot 0)
    (Math|Integer|IncrementInt (Variables|Default|GetCurrentFreeRowSlot))
    (else
      (Math|Integer|IncrementInt (Variables|Default|GetCurrentFreeColumnSlot)))))